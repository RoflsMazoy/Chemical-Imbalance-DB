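; Heat vent actor that thaws the player blob when it overlaps the vent.
; On overlap with a player-tagged BlobAnim_BP, it starts a looping fast timer that decrements the blob's FreezeLevel one step per tick.
; The timer clears itself once FreezeLevel reaches zero; leaving the vent does not stop it.
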(event `self.ReceiveActorBeginOverlap`
  (params (OtherActor :type "Actor Object Reference"))
  (bind _asblob_anim_bp (cast `/Game/Test_Blueprints/BlobAnim_BP` OtherActor))
  (if (`self.ActorHasTag` _asblob_anim_bp "player")
    (bind _returnvalue (`KismetSystemLibrary.K2_SetTimerDelegate` (delegate `Lower_freeze`) 0.05 true))
    (bind _output_get (set `self.vent_timer_stop` _returnvalue))))

(event `Lower_freeze`
  (if (== (`/Game/Test_Blueprints/BlobAnim_BP.FreezeLevel` (stale `self.ReceiveActorBeginOverlap` _asblob_anim_bp)) 0)
    (`KismetSystemLibrary.K2_ClearAndInvalidateTimerHandle` (stale `self.ReceiveActorBeginOverlap` _output_get))
    (else
      (set `/Game/Test_Blueprints/BlobAnim_BP.FreezeLevel` (- (`/Game/Test_Blueprints/BlobAnim_BP.FreezeLevel` (stale `self.ReceiveActorBeginOverlap` _asblob_anim_bp)) 1) (stale `self.ReceiveActorBeginOverlap` _asblob_anim_bp)))))

(fn `UserConstructionScript`)