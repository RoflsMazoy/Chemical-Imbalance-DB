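; Enemy AI character that wanders between random navmesh points, chases a player it sees and periodically performs a charge attack.
; PawnSensing sets the target, which is dropped when out of range or unseen for a timed period.
; Tick drives frame-scaled idle, target and charge countdowns feeding an integer state machine: follow, stop, face target, charge.
; The charge locks direction toward the target, then moves without sweeping until its timer returns it to following.
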(event `self.ReceiveTick`
  (params (DeltaSeconds :type "Float (single-precision)"))
  (bind _returnvalue (`self.GetTransform` (`self.Target`)))
  (bind _returnvalue_2 (`self.GetTransform` self))
  ;[1 1 1] Move around randomly while idling between moves
  (set `self.FrameTime` (* DeltaSeconds 60.0))
  (`self.IdleTimerTick`)
  (`self.TargetTimerTick`)
  (`self.ChargeTimerTick`)
  (if (and (not (`self.IsIdle`)) (not (`self.IsTarget`)) (not (`self.IsMoving`)) (== (`self.ChargeState`) 0))
    (`|AIMoveTo` self (`NavigationSystemV1.K2_GetRandomLocationInNavigableRadius` (`self.K2_GetActorLocation`) 3000.0 null null) null
      (:`then`
        (set `self.IsMoving` true))
      (:`OnSuccess`
        (set `self.IsMoving` false :!label _label)
        (`self.IdleTimerStart`))
      (:`OnFail`
        (goto _label)))
    (else
      ;[1 1 1] Check if targeting
      (if (`self.IsTarget`)
        (if (> (`self.GetDistanceTo` self (`self.Target`)) (`self.TargetDist`))
          (`self.ResetAI`)
          (else
            (switch `int` (`self.ChargeState`)
              (:`0`
                ;[1 1 1] Follow the target
                (`self.ChargeTimerStart`)
                (`|AIMoveTo` self (0.0 0.0 0.0) (`self.Target`) :!label _label_2))
              (:`1`
                (goto _label_2))
              (:`2`
                ;[1 1 1] Stop enermy moving and telemark the coming attack
                (`PrimitiveComponent.SetMaterial` (`self.Mesh`) 0 null)
                (`NavMovementComponent.StopActiveMovement` (`self.CharacterMovement`))
                (set `self.ChargeState` 3)
                (`self.ChargeTimerStart`))
              (:`3`
                ;[1 1 1] Rotate to look at target
                (`SceneComponent.K2_SetRelativeRotation` (`self.CapsuleComponent`) (`KismetMathLibrary.FindLookAtRotation` (`KismetMathLibrary.MakeVector` (.x (.location _returnvalue_2)) (.y (.location _returnvalue_2))) (`KismetMathLibrary.MakeVector` (.x (.location _returnvalue)) (.y (.location _returnvalue)))) false false))
              (:`4`
                ;[1 1 1] Charge in the last recorded direciton
                (`MovementComponent.K2_MoveUpdatedComponent` (`self.CharacterMovement`) (* (`self.ChargeDir`) (* (`self.ChargeSpd`) (`self.FrameTime`))) (`SceneComponent.RelativeRotation` (`self.CapsuleComponent`)) false false)))))))))

(event `self.PawnSensing.OnSeePawn`
  (params (Pawn :type "Pawn Object Reference"))
  ;[1 1 1] Check if there is a target in vision
  (set `self.IsTarget` (`self.ActorHasTag` Pawn "player"))
  (set `self.Target` Pawn)
  (`self.TargetTimerStart`))

(fn `ChargeTimerStart`
  (bind _chargetimersetmaxfollow (`self.ChargeTimerSetMaxFollow`))
  (switch `int` (`self.ChargeState`)
    (:`0`
      ;[1 1 1] Set a random time for the enermy to follow the target
      (set `self.ChargeTimer` (`KismetMathLibrary.RandomFloatInRange` (* _chargetimersetmaxfollow 0.25) _chargetimersetmaxfollow))
      (set `self.ChargeState` 1))
    (:`3`
      (set `self.ChargeTimer` (`self.ChargeTimerSetAgro`)))
    (:`4`
      (set `self.ChargeTimer` (`self.ChargeTimerSetCharge`)))))

(fn `ChargeTimerTick`
  (bind _chargetimer (`self.ChargeTimer`))
  (bind _returnvalue (`self.GetTransform` (`self.Target`)))
  (bind _returnvalue_2 (`self.GetTransform` self))
  (if (> _chargetimer 0.0)
    (bind _output_get (set `self.ChargeTimer` (- _chargetimer (`self.FrameTime`))))
    (if (< _output_get 0.0)
      (bind _result (`/Engine/EditorBlueprintResources/StandardMacros.IncrementInt` (`self.ChargeState`))
        (:`  `
          (switch `int` _result
            (:`4`
              ;[1 1 1] Record the direction that the enermy is currently looking in
              (set `self.ChargeDir` (`KismetMathLibrary.GetDirectionUnitVector` (`KismetMathLibrary.MakeVector` (.x (.location _returnvalue_2)) (.y (.location _returnvalue_2))) (`KismetMathLibrary.MakeVector` (.x (.location _returnvalue)) (.y (.location _returnvalue)))))
              (`self.ChargeTimerStart`))
            (:`5`
              ;[1 1 1] Reset the enermy back to the following state
              (`PrimitiveComponent.SetMaterial` (`self.Mesh`) 0 null)
              (set `self.ChargeState` 0)
              (`self.ChargeTimerStart`))))))))

(fn `IdleTimerStart`
  (bind _idletimerset (`self.IdleTimerSet`))
  (set `self.IdleTimer` (`KismetMathLibrary.RandomFloatInRange` (* _idletimerset 0.25) _idletimerset))
  (set `self.IsIdle` true))

(fn `IdleTimerTick`
  (bind _idletimer (`self.IdleTimer`))
  (if (> _idletimer 0.0)
    (bind _output_get (set `self.IdleTimer` (- _idletimer (`self.FrameTime`))))
    (if (< _output_get 0.0)
      (set `self.IsIdle` false))))

(fn `ResetAI`
  ;[1 1 1] Reset the AI back to wandering
  (`NavMovementComponent.StopActiveMovement` (`self.CharacterMovement`))
  (set `self.TargetTimer` -1.0)
  (set `self.ChargeTimer` -1.0)
  (set `self.IsTarget` false)
  (set `self.IsMoving` false)
  (set `self.ChargeState` 0)
  (`PrimitiveComponent.SetMaterial` (`self.Mesh`) 0 null)
  (`self.IdleTimerStart`))

(fn `TargetTimerStart`
  (set `self.TargetTimer` (`self.TargetTimerSet`))
  (set `self.IsIdle` true))

(fn `TargetTimerTick`
  (bind _targettimer (`self.TargetTimer`))
  (if (> _targettimer 0.0)
    (bind _output_get (set `self.TargetTimer` (- _targettimer (`self.FrameTime`))))
    (if (< _output_get 0.0)
      (set `self.IsTarget` false))))

(fn `UserConstructionScript`)