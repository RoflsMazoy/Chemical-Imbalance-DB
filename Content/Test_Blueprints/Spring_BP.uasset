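; Test spring actor that visually compresses its base mesh to follow the position of its Tip component.
; Each Tick, while the Tip's relative Z is below its rest height, it scales Basemodel's Z by the ratio of current to rest height, with fixed X and Y scale.
; The scale is left untouched at or above rest height, and nothing in this graph moves the Tip.
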(event `self.ReceiveBeginPlay`)

(event `self.ReceiveTick`
  (params (DeltaSeconds :type "Float (single-precision)"))
  (bind _returnvalue (`SceneComponent.GetRelativeTransform` (`self.tip`)))
  (if (< (.z (.location _returnvalue)) (`self.tiprestz`))
    (`SceneComponent.SetRelativeScale3D` (`self.basemodel`) (`KismetMathLibrary.MakeVector` 4.0 4.0 (* (`self.baserestz`) (/ (.z (.location _returnvalue)) (`self.tiprestz`)))))))

(fn `UserConstructionScript`)