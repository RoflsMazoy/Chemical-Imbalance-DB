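; Guidance trigger in the cave that shows an on-screen tip when the blob character overlaps its mesh with fewer than three collected keys.
; The tip text comes from the actor's first tag and fills a newly created Tips widget.
; An InRange counter prevents repeat popups until overlap end removes a valid widget after a delay and resets the count.
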(event `self.StaticMesh.OnComponentBeginOverlap`
  (params (OverlappedComponent :type "PrimitiveComponent Object Reference") (OtherActor :type "Actor Object Reference") (OtherComp :type "PrimitiveComponent Object Reference") (OtherBodyIndex :type Integer) (bFromSweep :type Boolean) (SweepResult :type "HitResult Structure (by ref)"))
  (bind _asblob_anim_bp (cast `/Game/Test_Blueprints/BlobAnim_BP` OtherActor))
  (set `self.InRange` (+ (`self.InRange`) 1))
  (if (< (`/Game/Test_Blueprints/BlobAnim_BP.CollectedKeys` _asblob_anim_bp) 3)
    (if (== (`self.InRange`) 1)
      (bind _returnvalue (`|CreateWidget` "/Game/Test_Levels/Test_Lab/Widgets/Tips.Tips_C"))
      (bind _output_get (set `self.TipsWidget` _returnvalue))
      (`self.SetTips` (`KismetTextLibrary.Conv_NameToText` (`|GetArrayItem` (`self.Tags`))))
      (`UserWidget.AddToViewport` _output_get 0))))

(event `self.StaticMesh.OnComponentEndOverlap`
  (params (OverlappedComponent :type "PrimitiveComponent Object Reference") (OtherActor :type "Actor Object Reference") (OtherComp :type "PrimitiveComponent Object Reference") (OtherBodyIndex :type Integer))
  (bind _tipswidget (`self.TipsWidget`))
  (cast `/Game/Test_Blueprints/BlobAnim_BP` OtherActor)
  (`KismetSystemLibrary.Delay` 20.0)
  (if (`KismetSystemLibrary.IsValid` _tipswidget)
    (`Widget.RemoveFromParent` _tipswidget)
    (set `self.InRange` 0)))

(fn `IsBlob`
  (params (Actor :type "Actor Object Reference"))
  (returns (Result :type Boolean))
  (return (== (`GameplayStatics.GetObjectClass` Actor) "/Game/Test_Blueprints/BlobAnim_BP.BlobAnim_BP_C")))

(fn `SetTips`
  (params (Text :type Text))
  (set `/Game/Test_Levels/Test_Lab/Widgets/Tips.Text` Text (`self.TipsWidget`)))

(fn `UserConstructionScript`)