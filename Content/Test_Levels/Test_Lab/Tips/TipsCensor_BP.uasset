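; TipsCensor_BP is a trigger actor that shows an on-screen tip while the blob character overlaps its static mesh.
; Begin overlap checks for an exact BlobAnim_BP class match, then creates a Tips widget, sets its text and adds it to the viewport.
; The tip text comes from the actor's first tag, so each placed instance can carry its own message.
; End overlap by the blob removes the widget.
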(event `self.StaticMesh.OnComponentBeginOverlap`
  (params (OverlappedComponent :type "PrimitiveComponent Object Reference") (OtherActor :type "Actor Object Reference") (OtherComp :type "PrimitiveComponent Object Reference") (OtherBodyIndex :type Integer) (bFromSweep :type Boolean) (SweepResult :type "HitResult Structure (by ref)"))
  (bind _result (`self.IsBlob` OtherActor))
  (if _result
    (bind _returnvalue (`|CreateWidget` "/Game/Test_Levels/Test_Lab/Widgets/Tips.Tips_C"))
    (bind _output_get (set `self.TipsWidget` _returnvalue))
    (`self.SetTips` (`KismetTextLibrary.Conv_NameToText` (`|GetArrayItem` (`self.Tags`))))
    (`UserWidget.AddToViewport` _output_get 0)))

(event `self.StaticMesh.OnComponentEndOverlap`
  (params (OverlappedComponent :type "PrimitiveComponent Object Reference") (OtherActor :type "Actor Object Reference") (OtherComp :type "PrimitiveComponent Object Reference") (OtherBodyIndex :type Integer))
  (bind _result (`self.IsBlob` OtherActor))
  (if _result
    (`Widget.RemoveFromParent` (`self.TipsWidget`))))

(fn `IsBlob`
  (params (Actor :type "Actor Object Reference"))
  (returns (Result :type Boolean))
  (return (== (`GameplayStatics.GetObjectClass` Actor) "/Game/Test_Blueprints/BlobAnim_BP.BlobAnim_BP_C")))

(fn `SetTips`
  (params (Text :type Text))
  (set `/Game/Test_Levels/Test_Lab/Widgets/Tips.Text` Text (`self.TipsWidget`)))

(fn `UserConstructionScript`)