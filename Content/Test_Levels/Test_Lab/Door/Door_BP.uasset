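; Test-lab double door actor that toggles open and closed each time an actor begins overlapping it.
; ChangeState snaps the two side pivots between closed and 90-degree yaw, swaps the light and button materials to match, and flips IsOpen.
; ChangeDecal then sets the link decal to glow yellow when open or look off when closed, affecting only the first Powered_decal actor found in the level.
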(event `self.ReceiveActorBeginOverlap`
  (params (OtherActor :type "Actor Object Reference"))
  ;[1 1 1] Door opening code
  (`self.ChangeState` (`self.IsOpen`))
  (`self.ChangeDecal`))

(event `self.Button.OnComponentHit`
  (params (HitComponent :type "PrimitiveComponent Object Reference") (OtherActor :type "Actor Object Reference") (OtherComp :type "PrimitiveComponent Object Reference") (NormalImpulse :type "Vector Structure") (Hit :type "HitResult Structure (by ref)")))

(fn `ChangeDecal`
  ;[1 1 1] Gets all actors of class link decal, returns the first of them in the scene
  (bind _outactors (`GameplayStatics.GetAllActorsOfClass` "/Game/Test_Levels/Test_Lab/Door/powered_decal.powered_decal_C"))
  (bind _output (`|GetArrayItem` _outactors))
  (cast `Actor` _output)
  (if (`self.IsOpen`)
    (bind _link_decal (`/Game/Test_Levels/Test_Lab/Door/powered_decal.link_decal` _output))
    (`PrimitiveComponent.SetMaterial` _link_decal 0 "/Game/Test_Levels/Test_Lab/Door/YellowGlow.YellowGlow")
    (else
      (`PrimitiveComponent.SetMaterial` _link_decal 0 "/Game/Test_Levels/Test_Lab/touch_button/link_decal_texture_off.link_decal_texture_off"))))

(fn `ChangeState`
  (params (Open :type Boolean))
  (bind _button (`self.Button`))
  (if Open
    (`SceneComponent.K2_SetRelativeRotation` :`self` (`self.SceneL`))
    (`SceneComponent.K2_SetRelativeRotation` :`self` (`self.SceneR`))
    (`PrimitiveComponent.SetMaterial` (`self.Light`) 0 "/Game/Test_Levels/Test_Lab/Door/RedGlow.RedGlow")
    (`PrimitiveComponent.SetMaterial` _button 0 "/Game/Test_Levels/Test_Lab/touch_button/soft_button_text_off.soft_button_text_off")
    (set `self.IsOpen` false)
    (else
      (`SceneComponent.K2_SetRelativeRotation` (`self.SceneL`) (struct :`Yaw` -90.0) false false)
      (`SceneComponent.K2_SetRelativeRotation` (`self.SceneR`) (struct :`Yaw` 90.0) false false)
      (`PrimitiveComponent.SetMaterial` (`self.Light`) 0 "/Game/Test_Levels/Test_Lab/Door/GreenGlow.GreenGlow")
      (`PrimitiveComponent.SetMaterial` _button 0 "/Game/Test_Levels/Test_Lab/touch_button/soft_button_text_on.soft_button_text_on")
      (set `self.IsOpen` true))))

(fn `UserConstructionScript`)