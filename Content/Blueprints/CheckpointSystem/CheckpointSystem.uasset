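; Checkpoint manager that saves checkpoint progress per level and respawns the blob at the last checkpoint.
; On BeginPlay it gathers the level's checkpoints and first blob, restores active flags from CI_GameInstance by object name, then teleports the blob, zeroing its linear velocity.
; Update records a new last checkpoint, adds it to the active list and writes both to the game instance under the current level name.
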(event `self.ReceiveBeginPlay`
  (bind _lastcheckpoint (`self.LastCheckpoint`))
  (`self.GetCPsFromLevel`)
  (`self.GetGameInstance`)
  (`self.GetCPs`)
  (`self.GetBlob`)
  (if (`KismetSystemLibrary.IsValid` _lastcheckpoint)
    (`self.Teleport` _lastcheckpoint)))

(fn `GetBlob`
  ;[1 1 1] Retrieve the first blob instance
  (bind _outactors (`GameplayStatics.GetAllActorsOfClass` "/Game/Test_Blueprints/BlobAnim_BP.BlobAnim_BP_C"))
  (set `self.Blob` (`|GetArrayItem` _outactors)))

(fn `GetCPs`
  ;[1 1 1] Retrieve active checkpoints and last checkpoint of current level from game instance
  (bind _returnvalue (`GameplayStatics.GetCurrentLevelName` true))
  (bind (_acps _lcp) (`/Game/Blueprints/CheckpointSystem/CI_GameInstance.RetrieveCPs` (`self.GameInstance`) _returnvalue))
  ;[1 1 1] Check data existence
  (if (!= (`KismetArrayLibrary.Array_Length` _acps) 0)
    ;[1 1 1] Activate checkpoints if exist in active checkpoints array
    (for _array_element (`self.Checkpoints`)
      (bind _returnvalue_2 (`KismetSystemLibrary.GetObjectName` _array_element))
      (if (`KismetArrayLibrary.Array_Contains` _acps _returnvalue_2)
        (set `/Game/Blueprints/CheckpointSystem/Checkpoint_BP.IsActive` true _array_element)
        ;[1 1 1] Setup last checkpoint
        (if (`KismetStringLibrary.EqualEqual_StrStr` _returnvalue_2 _lcp)
          (set `self.LastCheckpoint` _array_element))))))

(fn `GetCPsFromLevel`
  ;[1 1 1] Retrieve all checkpoint from current level
  (bind _outactors (`GameplayStatics.GetAllActorsOfClass` "/Game/Blueprints/CheckpointSystem/Checkpoint_BP.Checkpoint_BP_C"))
  (set `self.Checkpoints` _outactors))

(fn `GetGameInstance`
  (bind _asci_game_instance (cast `/Game/Blueprints/CheckpointSystem/CI_GameInstance` (`GameplayStatics.GetGameInstance`)))
  (set `self.GameInstance` _asci_game_instance))

(fn `SetCPs`
  ;[1 1 1] Update checkpoints information to game instance
  (bind _returnvalue (`GameplayStatics.GetCurrentLevelName` true))
  (`/Game/Blueprints/CheckpointSystem/CI_GameInstance.UpdateCPs` (`self.GameInstance`) (`KismetSystemLibrary.GetObjectName` (`self.LastCheckpoint`)) _returnvalue (`self.ActiveCheckpoints`)))

(fn `Teleport`
  (params (TargetCheckpoint :type "/Game/Blueprints/CheckpointSystem/Checkpoint_BP Object Reference"))
  ;[1 1 1] Teleport the blob to target checkpoint  TODO: stop movement after teleport
  (`self.K2_TeleportTo` :`self` (`self.Blob`) :`DestLocation` (`SceneComponent.K2_GetComponentLocation` (`/Game/Blueprints/CheckpointSystem/Checkpoint_BP.StaticMesh` TargetCheckpoint)))
  (`PrimitiveComponent.SetPhysicsLinearVelocity` (`/Game/Test_Blueprints/BlobAnim_BP.Character_Collision` (`self.Blob`)) (0.0 0.0 0.0) false "None"))

(fn `Update`
  (params (LastCheckPoint :type "/Game/Blueprints/CheckpointSystem/Checkpoint_BP Object Reference"))
  (bind _activecheckpoints (`self.ActiveCheckpoints`))
  ;[1 1 1] Update last check point and active checkpoints array, then update to game instance
  (bind _output_get (set `self.LastCheckpoint` LastCheckPoint))
  (bind _returnvalue (`KismetSystemLibrary.GetObjectName` _output_get))
  (if (not (`KismetArrayLibrary.Array_Contains` _activecheckpoints _returnvalue))
    (`KismetArrayLibrary.Array_Add` _activecheckpoints _returnvalue))
  (`self.SetCPs`))

(fn `UserConstructionScript`)