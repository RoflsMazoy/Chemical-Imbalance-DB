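; Game instance for the checkpoint system that keeps checkpoint records per level.
; UpdateCPs finds the record matching the level name, or constructs a 2DArray_CPs object and adds it to the CPs array, with UpdateCP writing the LCP and ACPs values.
; RetrieveCPs searches the array by level name and returns the stored values.
; Wrapper objects give the array nested per-level data; NewFunction_0 is an empty stub.
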(fn `NewFunction_0`
  (params (NewParam :type "Array of String (by ref)")))

(fn `RetrieveCPs`
  (params (LevelName :type String))
  (returns (ACPs :type "Array of String") (LCP :type String))
  ;[1 1 1] Retrieve check point data if exists
  (for _array_element (`self.CPs`)
    (if (`KismetStringLibrary.EqualEqual_StrStr` LevelName (`/Game/Blueprints/CheckpointSystem/2DArray_CPs.LevelName` _array_element))
      (return (`/Game/Blueprints/CheckpointSystem/2DArray_CPs.ACPs` _array_element) (`/Game/Blueprints/CheckpointSystem/2DArray_CPs.LCP` _array_element)))))

(fn `UpdateCP`
  (params (LevelName :type String) (CP :type "/Game/Blueprints/CheckpointSystem/2DArray_CPs Object Reference (by ref)") (LCP :type String) (ACPs :type "Array of String"))
  (bind _cp (`local.CP`))
  ;[1 1 1] Check whether CP is a default instance
  (if (not (`KismetStringLibrary.NotEqual_StrStr` (`/Game/Blueprints/CheckpointSystem/2DArray_CPs.LevelName` CP)))
    ;[1 1 1] Setup variables
    (set `/Game/Blueprints/CheckpointSystem/2DArray_CPs.LevelName` (`local.LevelName`) _cp))
  (set `/Game/Blueprints/CheckpointSystem/2DArray_CPs.LCP` (`local.LCP`) _cp)
  (set `/Game/Blueprints/CheckpointSystem/2DArray_CPs.ACPs` (`local.ACPs`) _cp))

(fn `UpdateCPs`
  (params (LCP :type String) (LevelName :type String) (ACPs :type "Array of String"))
  ;[1 1 1] Check level information existence
  (for (_array_element _array_index) (`self.CPs`)
    (if (`KismetStringLibrary.EqualEqual_StrStr` (`local.LevelName`) (`/Game/Blueprints/CheckpointSystem/2DArray_CPs.LevelName` _array_element))
      ;[1 1 1] Update exist checkpoint
      (`self.UpdateCP` "" (`|GetArrayItem` (`self.CPs`) _array_index) (`local.LCP`) (`local.ACPs`))
      (return)))
  ;[1 1 1] Create record instance and add to game instance
  (bind _returnvalue (`|GenericCreateObject` "/Game/Blueprints/CheckpointSystem/2DArray_CPs.2DArray_CPs_C" "CI_GameInstance"))
  (`self.UpdateCP` (`local.LevelName`) _returnvalue (`local.LCP`) (`local.ACPs`))
  (`KismetArrayLibrary.Array_Add` (`self.CPs`) _returnvalue)
  (return))