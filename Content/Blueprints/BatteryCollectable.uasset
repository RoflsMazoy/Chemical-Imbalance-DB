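; Battery pickup that recharges the player's flashlight in BlobAnim_BP when an actor overlaps it.
; On overlap it casts the player pawn, not the overlapping actor, adds its Value to FlashlightBattery and caps the result at 100.
; It then hands off to the parent class's overlap handler, which is skipped if the cast fails.
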(event `self.ReceiveActorBeginOverlap`
  (params (OtherActor :type "Actor Object Reference"))
  (bind _asblob_anim_bp (cast `/Game/Test_Blueprints/BlobAnim_BP` (`GameplayStatics.GetPlayerPawn` 0)))
  (bind _output_get (set `/Game/Test_Blueprints/BlobAnim_BP.FlashlightBattery` (+ (`/Game/Test_Blueprints/BlobAnim_BP.FlashlightBattery` _asblob_anim_bp) (`self.Value`)) _asblob_anim_bp))
  (if (> _output_get 100.0)
    (set `/Game/Test_Blueprints/BlobAnim_BP.FlashlightBattery` 100.0 _asblob_anim_bp))
  (`parent.ReceiveActorBeginOverlap` OtherActor))

(fn `UserConstructionScript`
  (`parent.UserConstructionScript`))