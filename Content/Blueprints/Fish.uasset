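; Fish Blueprint whose mesh travels along a spline path when a BlobAnim_BP actor overlaps its collision component.
; The overlap plays the MovingPlatform timeline, whose TravelDistance track is scaled by the spline's length to get a distance along the path.
; Each update sets the mesh's world location and relative rotation from the spline at that distance, without sweeping.
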(event `self.Collision.OnComponentBeginOverlap`
  (params (OverlappedComponent :type "PrimitiveComponent Object Reference") (OtherActor :type "Actor Object Reference") (OtherComp :type "PrimitiveComponent Object Reference") (OtherBodyIndex :type Integer) (bFromSweep :type Boolean) (SweepResult :type "HitResult Structure (by ref)"))
  (bind _spline (`self.Spline`))
  (cast `/Game/Test_Blueprints/BlobAnim_BP` OtherActor)
  (bind (_direction _travel_distance) (`Timeline|MovingPlatform`)
    (:`Update`
      (bind _returnvalue (* _travel_distance (`SplineComponent.GetSplineLength` (`self.Spline`))))
      (`SceneComponent.K2_SetWorldLocation` (`self.Mesh`) (`SplineComponent.GetLocationAtDistanceAlongSpline` _spline _returnvalue "World") false false)
      (`SceneComponent.K2_SetRelativeRotation` (`self.Mesh`) (`SplineComponent.GetRotationAtDistanceAlongSpline` _spline _returnvalue "Local") false false))))

(fn `UserConstructionScript`)