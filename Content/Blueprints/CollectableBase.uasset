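; Base collectable actor that the player picks up by touching it.
; On overlap with an actor tagged Player, it casts to BlobAnim_BP, increments its GeneralCollTotal, then destroys itself after a short delay.
; Each tick it spins on its yaw axis at a RotatePerSecond rate, scaled by delta time.
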(event `self.ReceiveActorBeginOverlap`
  (params (OtherActor :type "Actor Object Reference"))
  ;[1 1 1] Disappear when picked up
  (if (`self.ActorHasTag` OtherActor "Player")
    (bind _asblob_anim_bp (cast `/Game/Test_Blueprints/BlobAnim_BP` OtherActor))
    (set `/Game/Test_Blueprints/BlobAnim_BP.GeneralCollTotal` (+ (`/Game/Test_Blueprints/BlobAnim_BP.GeneralCollTotal` _asblob_anim_bp) 1) _asblob_anim_bp)
    (`KismetSystemLibrary.Delay` 0.2)
    (`self.K2_DestroyActor`)))

(event `self.ReceiveTick`
  (params (DeltaSeconds :type "Float (single-precision)"))
  ;[1 1 1] Spin on the Spot
  (`self.K2_AddActorLocalRotation` (`KismetMathLibrary.MakeRotator` 0.0 0.0 (* DeltaSeconds (`self.RotatePerSecond`)))))

(fn `UserConstructionScript`)