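; Instanced foliage tree component that swaps a hit tree instance for an actor tree that receives the shake.
; On BeginPlay it pre-spawns a pool of ActorTree actors far below the world.
; A strong enough normal impulse, or a direct float hit, moves an inactive pooled actor onto the instance's transform and initializes it with hit data.
; The instance is hidden by offsetting its location, and Reset adds that offset back.
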(event `self.ReceiveBeginPlay`
  (bind _actortrees (`self.ActorTrees`))
  (for (_ _array_index) _actortrees
    (bind _returnvalue (`|SpawnActorFromClass` (`self.TreeType`) (`KismetMathLibrary.MakeTransform` (0.0 0.0 -10000.0)) "Undefined" "OverrideRootScale" null null))
    (bind _asactor_tree (cast `/Game/Blueprints/Terrain/ActorTree` _returnvalue)
      (:`then`
        (`KismetArrayLibrary.Array_Set` _actortrees _array_index _asactor_tree))
      (:`CastFailed`
        (`KismetSystemLibrary.PrintString` "failed actor tree cast")))))

(fn `Float Hit`
  (params (Index :type Integer) (`Shake Power` :type "Float (double-precision)") (`Hit Normal X` :type "Float (double-precision)") (`Hit Normal Y` :type "Float (double-precision)"))
  (bind _outinstancetransform (`self.GetInstanceTransform` Index))
  (bind _actortree (`self.GetActorTree` _outinstancetransform))
  (`/Game/Blueprints/Terrain/ActorTree.Initialize` _actortree `Hit Normal X` `Hit Normal Y` `Shake Power` self Index)
  (`self.UpdateInstanceTransform` Index (`KismetMathLibrary.MakeTransform` (- (.location _outinstancetransform) (`self.HideMove`)) (.rotation _outinstancetransform) (.scale _outinstancetransform))))

(fn `GetActorTree`
  (params (`Instance Transform` :type "Transform Structure"))
  (returns (ActorTree :type "/Game/Blueprints/Terrain/ActorTree Object Reference"))
  (for _array_element (`self.ActorTrees`)
    (if (not (`/Game/Blueprints/Terrain/ActorTree.Active` _array_element))
      (set `/Game/Blueprints/Terrain/ActorTree.Active` true _array_element)
      (`Actor.K2_SetActorTransform` _array_element `Instance Transform` false false)
      (return _array_element)))
  (return null))

(fn `Normal Hit`
  (params (Index :type Integer) (`Normal Impluse` :type "Vector Structure") (`Hit Normal X` :type "Float (double-precision)") (`Hit Normal Y` :type "Float (double-precision)"))
  (if (> (/ (`KismetMathLibrary.VSize` `Normal Impluse`) (`self.shakedivider`)) (`self.shakethreshold`))
    (`self.Float Hit` Index 9.0 `Hit Normal X` `Hit Normal Y`)))

(fn `Reset`
  (params (`Instance Index` :type Integer))
  (`self.UpdateInstanceTransform` `Instance Index` (`KismetMathLibrary.MakeTransform` (+ (.location (`self.GetInstanceTransform` `Instance Index`)) (`self.HideMove`)) (.rotation (`self.GetInstanceTransform` `Instance Index`)) (.scale (`self.GetInstanceTransform` `Instance Index`)))))