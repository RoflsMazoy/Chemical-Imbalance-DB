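; Stand-in tree actor that shakes when hit, dropping leaves and playing a random twang sound, in place of a foliage tree instance.
; Initialize turns a pivot to the hit normal and reparents the mesh under it, so the sway follows the hit direction.
; Tick swings the pitch back and forth with decaying, frame-time-scaled motion.
; After the leaf timer, it moves itself away and resets the FoilageTree instance.
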(event `self.ReceiveTick`
  (params (DeltaSeconds :type "Float (single-precision)"))
  (bind _currenty (`self.currentY`))
  (bind _returnvalue (- (`self.shakepower`) (`self.shakedecay`)))
  (bind _returnvalue_2 (* (`self.shakespeed`) (`self.frametime`)))
  (bind _output_get (set `self.frametime` (* DeltaSeconds 60.0)))
  (if (> (`self.shakepower`) 0.0)
    (if (`self.negativerotation`)
      (set `self.currentY` (- _currenty _returnvalue_2))
      (else
        (set `self.currentY` (+ _currenty _returnvalue_2))))
    (`SceneComponent.K2_SetRelativeRotation` (`self.RotY`) (`KismetMathLibrary.MakeRotator` 0.0 (`self.currentY`)) false false)
    (if (< (`self.currentY`) (* (`self.shakepower`) -1.0))
      (bind _output_get_2 (set `self.shakepower` _returnvalue))
      (set `self.currentY` (* _output_get_2 -1.0))
      (if (`self.negativerotation`) :!label _label
        (set `self.negativerotation` false)
        (else
          (set `self.negativerotation` true)))
      (elif (> (`self.currentY`) (`self.shakepower`))
        (bind _output_get_3 (set `self.shakepower` _returnvalue))
        (set `self.currentY` _output_get_3)
        (goto _label)))
    (elif (< (`self.emittimer`) (`self.emittimerlimit`))
      (set `self.emittimer` (+ (`self.emittimer`) _output_get))
      (elif (`self.emittiming`)
        (`ActorComponent.Deactivate` (`self.FallingLeaves`))
        (set `self.emittiming` false)
        (set `self.Active` false)
        (`self.K2_SetActorTransform` (`KismetMathLibrary.MakeTransform` (* (`/Game/Blueprints/Terrain/FoilageTree.HideMove` (`self.FoilageTree`)) -1.0)))
        (`/Game/Blueprints/Terrain/FoilageTree.Reset` (`self.FoilageTree`) (`self.Instance Index`))))))

(fn `GetTwangSound`
  (returns (Sound :type "SoundWave Object Reference"))
  (switch `int` (`KismetMathLibrary.RandomIntegerInRange` 0 3)
    (:`0`
      (return "/Game/Sounds/Tree_Twang/tree_twang_1.tree_twang_1"))
    (:`1`
      (return "/Game/Sounds/Tree_Twang/tree_twang_2.tree_twang_2"))
    (:`2`
      (return "/Game/Sounds/Tree_Twang/tree_twang_3.tree_twang_3"))
    (:`3`
      (return "/Game/Sounds/Tree_Twang/tree_twang_4.tree_twang_4"))))

(fn `Initialize`
  (params (`Hit Normal X` :type "Float (double-precision)") (`Hit Normal Y` :type "Float (double-precision)") (`Shake Power` :type "Float (double-precision)") (FoilageTree :type "/Game/Blueprints/Terrain/FoilageTree Object Reference") (`Instance Index` :type Integer))
  (bind _twangsound (`self.TwangSound`))
  (set `self.FoilageTree` FoilageTree)
  (set `self.Instance Index` `Instance Index`)
  (set `self.shakepower` `Shake Power`)
  (`SceneComponent.K2_DetachFromComponent` (`self.TreeMesh`) "KeepWorld" "KeepWorld" "KeepWorld" true)
  (`SceneComponent.K2_SetWorldRotation` (`self.RotZ`) (`KismetMathLibrary.Conv_VectorToRotator` (`KismetMathLibrary.MakeVector` (* `Hit Normal X` -1.0) (* `Hit Normal Y` -1.0))) false false)
  (`SceneComponent.K2_AttachToComponent` (`self.TreeMesh`) (`self.RotY`) "None" "KeepWorld" "KeepWorld" "KeepWorld" true)
  (set `self.negativerotation` false)
  (`ActorComponent.Activate` (`self.FallingLeaves`) false)
  (set `self.emittiming` true)
  (set `self.emittimer` 0.0)
  (`AudioComponent.SetSound` _twangsound (`self.GetTwangSound`))
  (`AudioComponent.Play` _twangsound 0.0))

(fn `UserConstructionScript`)